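; BP_Car is a drivable vehicle pawn that the player controls and can exit.
; On possession it replaces the local player's input mappings with IMC_Driver, whose throttle, brake, steering and handbrake actions feed the VehicleMovementComponent on both trigger and completion.
; Legacy mouse axis events orbit and zoom the Boom camera component.
; The hardcoded F key has CarSeat kick the BP_Driver found in the level out to the Arrow exit point.
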(event `self.ReceivePossessed`
  (params (NewController :type "Controller Object Reference"))
  (bind _returnvalue (pcsubsystem `EnhancedInputLocalPlayerSubsystem` (`GameplayStatics.GetPlayerController` 0)))
  (`EnhancedInputSubsystemInterface.ClearAllMappings` _returnvalue)
  (`EnhancedInputSubsystemInterface.AddMappingContext` _returnvalue "/Game/C4F_Driver/Inputs/IMC_Driver.IMC_Driver" 0 (struct)))

(event `EnhancedInput|/Game/C4F_Driver/Inputs/IA_Accel`
  (params (ActionValue :type "Float (double-precision)") (ElapsedSeconds :type "Float (double-precision)") (TriggeredSeconds :type "Float (double-precision)") (InputAction :type "InputAction Object Reference" :default "/Game/C4F_Driver/Inputs/IA_Accel.IA_Accel"))
  (:`Triggered`
    (`ChaosVehicleMovementComponent.SetThrottleInput` (`self.VehicleMovementComponent`) ActionValue :!label _label))
  (:`Completed`
    (goto _label)))

(event `EnhancedInput|/Game/C4F_Driver/Inputs/IA_Brake`
  (params (ActionValue :type "Float (double-precision)") (ElapsedSeconds :type "Float (double-precision)") (TriggeredSeconds :type "Float (double-precision)") (InputAction :type "InputAction Object Reference" :default "/Game/C4F_Driver/Inputs/IA_Brake.IA_Brake"))
  (:`Triggered`
    (`ChaosVehicleMovementComponent.SetBrakeInput` (`self.VehicleMovementComponent`) ActionValue :!label _label_2))
  (:`Completed`
    (goto _label_2)))

(event `InputAxisKey|MouseX`
  (params (AxisValue :type "Float (single-precision)"))
  (`Boom.Orbit` (`self.Boom`) AxisValue (stale `InputAxisKey|MouseY` AxisValue) :!label _label_3))

(event `EnhancedInput|/Game/C4F_Driver/Inputs/IA_Steer`
  (params (ActionValue :type "Float (double-precision)") (ElapsedSeconds :type "Float (double-precision)") (TriggeredSeconds :type "Float (double-precision)") (InputAction :type "InputAction Object Reference" :default "/Game/C4F_Driver/Inputs/IA_Steer.IA_Steer"))
  (:`Triggered`
    (`ChaosVehicleMovementComponent.SetSteeringInput` (`self.VehicleMovementComponent`) ActionValue :!label _label_4))
  (:`Completed`
    (goto _label_4)))

(event `InputAxisKey|MouseY`
  (params (AxisValue :type "Float (single-precision)"))
  (goto _label_3))

(event `InputAxisKey|MouseWheelAxis`
  (params (AxisValue :type "Float (single-precision)"))
  (`Boom.Zoom` (`self.Boom`) AxisValue))

(event `EnhancedInput|/Game/C4F_Driver/Inputs/IA_Handbrake`
  (params (ActionValue :type Boolean) (ElapsedSeconds :type "Float (double-precision)") (TriggeredSeconds :type "Float (double-precision)") (InputAction :type "InputAction Object Reference" :default "/Game/C4F_Driver/Inputs/IA_Handbrake.IA_Handbrake"))
  (:`Triggered`
    (`ChaosVehicleMovementComponent.SetHandbrakeInput` (`self.VehicleMovementComponent`) ActionValue :!label _label_5))
  (:`Completed`
    (goto _label_5)))

(event `Key|F`
  (params (Key :type "Key Structure"))
  (:`Pressed`
    (bind _returnvalue (`GameplayStatics.GetActorOfClass` "/Game/C4F_Driver/Blueprints/BP_Driver.BP_Driver_C"))
    (`CarSeat.KickOccupant` (`self.CarSeat`) _returnvalue (`self.Arrow`))))

(fn `UserConstructionScript`)